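; Door Blueprint that swings open by itself once the player character's lock is broken.
; BeginPlay caches the BP_ThirdPersonCharacter; Tick polls its LockBroken flag, sets and prints DoorOpenable, then calls DoorOpen every frame.
; When openable, DoorOpen drives a Timeline that lerps the door's yaw through a quarter turn.
; A DoOnce with no reset precedes the FlipFlop, so the reverse (closing) branch is never reached.
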(event Custom|DoorOpen
  (if (Variables|Default|GetDoorOpenable)
    (Utilities|FlowControl|DoOnce false
      (:Completed
        (Utilities|FlowControl|FlipFlop
          (:A
            (bind _door_float (Timeline|Timeline PlayFromStart)
              (:Update
                (Transformation|SetRelativeRotation (Variables|Default|GetDoor) (Math|Rotator|MakeRotator 0.0 0.0 (Math|Float|Lerp 0.0 9e+01 _door_float)) false false))))
          (:B
            (Timeline|Timeline Reverse)))))))

(event EventBeginPlay
  (bind _asbp_third_person_character (Utilities|Casting|CastToBP_ThirdPersonCharacter (Game|GetPlayerCharacter 0)))
  (Variables|Default|SetAs%20BP%20Third%20Person%20Character _asbp_third_person_character))

(event EventTick
  (params (DeltaSeconds :type Float%20%28single-precision%29))
  (Utilities|FlowControl|Sequence
    (:then_0
      (if (Variables|/Game/ThirdPerson/Blueprints/BP_ThirdPersonCharacter.BP_ThirdPersonCharacter_C|GetLockBroken (Variables|Default|GetAs%20BP%20Third%20Person%20Character))
        (bind _output_get (Variables|Default|SetDoorOpenable true))
        (Development|PrintText (Utilities|Text|ToText(Boolean) _output_get))))
    (:then_1
      (CallFunction|DoorOpen))))

(fn ConstructionScript)