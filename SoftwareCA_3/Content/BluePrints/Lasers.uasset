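; Laser hazard actor that kills the player on touch.
; On BeginPlay it casts player 0's character to BP_ThirdPersonCharacter and caches the reference.
; Overlap with an actor tagged Player sets IsDead and calls Death on that cached character, rather than on the overlapping actor.
; Overlap with an actor tagged Lava destroys the laser itself.
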(event EventBeginPlay
  (bind _asbp_third_person_character (Utilities|Casting|CastToBP_ThirdPersonCharacter (Game|GetPlayerCharacter 0)))
  (Variables|Default|SetAs%20BP%20Third%20Person%20Character _asbp_third_person_character))

(event Collision|EventActorBeginOverlap
  (params (OtherActor :type Actor%20Object%20Reference))
  (bind _as_bp_third_person_character (Variables|Default|GetAs%20BP%20Third%20Person%20Character))
  (Utilities|FlowControl|Sequence
    (:then_0
      (if (Actor|ActorHasTag OtherActor "Player")
        (Variables|/Game/ThirdPerson/Blueprints/BP_ThirdPersonCharacter.BP_ThirdPersonCharacter_C|SetIsDead _as_bp_third_person_character true)
        (Default|Death _as_bp_third_person_character)))
    (:then_1
      (if (Actor|ActorHasTag OtherActor "Lava")
        (Actor|DestroyActor)))))

(fn ConstructionScript)