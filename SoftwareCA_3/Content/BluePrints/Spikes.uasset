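; Spikes is a breakable obstacle actor that the player destroys by attacking it, which also flags a lock as broken.
; It caches the third-person character on BeginPlay.
; On overlap with a Player-tagged actor, it checks that character's IsAttacking flag, then destroys itself and sets LockBroken on the character.
; Overlap with a Lava-tagged actor also destroys it, without setting the flag.
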(event EventBeginPlay
  (Utilities|FlowControl|Sequence
    (:then_0
      (bind _asbp_third_person_character (Utilities|Casting|CastToBP_ThirdPersonCharacter (Game|GetPlayerCharacter 0)))
      (Variables|Default|SetAs%20BP%20Third%20Person%20Character _asbp_third_person_character))))

(event Collision|EventActorBeginOverlap
  (params (OtherActor :type Actor%20Object%20Reference))
  (Utilities|FlowControl|Sequence
    (:then_0
      (if (Actor|ActorHasTag OtherActor "Player")
        (if (Variables|/Game/ThirdPerson/Blueprints/BP_ThirdPersonCharacter.BP_ThirdPersonCharacter_C|GetIsAttacking (Variables|Default|GetAs%20BP%20Third%20Person%20Character))
          (Actor|DestroyActor)
          (Variables|/Game/ThirdPerson/Blueprints/BP_ThirdPersonCharacter.BP_ThirdPersonCharacter_C|SetLockBroken (Variables|Default|GetAs%20BP%20Third%20Person%20Character) true))))
    (:then_1
      (if (Actor|ActorHasTag OtherActor "Lava")
        (Actor|DestroyActor)))))

(fn ConstructionScript)