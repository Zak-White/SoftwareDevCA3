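; LongLasers is a laser hazard Blueprint that kills the player on contact.
; It caches the BP_FirstPersonCharacter reference on BeginPlay.
; On overlap with an actor tagged Player, it sets IsDead on that cached character and calls Death.
; On overlap with an actor tagged Lava, the laser destroys itself.
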(event EventBeginPlay
  (bind _asbp_first_person_character (Utilities|Casting|CastToBP_FirstPersonCharacter (Game|GetPlayerCharacter 0)))
  (Variables|Default|SetAs%20BP%20First%20Person%20Character _asbp_first_person_character))

(event Collision|EventActorBeginOverlap
  (params (OtherActor :type Actor%20Object%20Reference))
  (Utilities|FlowControl|Sequence
    (:then_0
      (if (Actor|ActorHasTag OtherActor "Player")
        (Variables|/Game/FirstPerson/Blueprints/BP_FirstPersonCharacter.BP_FirstPersonCharacter_C|SetIsDead (Variables|Default|GetAs%20BP%20First%20Person%20Character) true)
        (Default|Death (Variables|Default|GetAs%20BP%20First%20Person%20Character))))
    (:then_1
      (if (Actor|ActorHasTag OtherActor "Lava")
        (Actor|DestroyActor)))))

(fn ConstructionScript)